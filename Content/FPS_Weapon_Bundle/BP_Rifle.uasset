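; BP_Rifle is an automatic hitscan rifle with an ammo count and timed reload.
; StartShoot fires immediately and starts a looping Shoot timer, which StopShoot clears.
; Each shot uses ammo, plays a sound and traces from ShootSocket toward the camera's aim point, ignoring the attach parent, with debug drawing; hits spawn an explosion and apply point damage.
; Reload refills ammo after a retriggerable delay, then calls the OnReloaded dispatcher.
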(event Custom|Shoot
  (bind _returnvalue (Game|GetPlayerCameraManager 0))
  (bind _shootsocket (Variables|Default|GetShootSocket))
  (bind _returnvalue_2 (Transformation|GetWorldLocation _shootsocket))
  (if (> (Variables|Default|GetAmmo) 0)
    (Math|Integer|DecrementInt (Variables|Default|GetAmmo)
      (:%20%20
        (bind _outhit (Collision|LineTraceForObjects _returnvalue_2 (+ (Camera|GetCameraLocation _returnvalue) (* (Transformation|GetActorForwardVector _returnvalue) 20000)) (Utilities|Array|MakeArray "ObjectTypeQuery1" "ObjectTypeQuery2" "ObjectTypeQuery3") false (Utilities|Array|MakeArray (Actor|GetAttachParentActor)) "ForDuration" true "(R=1.000000,G=0.000000,B=0.000000,A=1.000000)" "(R=0.000000,G=1.000000,B=0.000000,A=1.000000)" 1.0))
        (Audio|PlaySoundatLocation 0 _returnvalue_2 "0, 0, 0" 1.0 1.0 0.0 0 0 0 0)
        (if (.bBlockingHit (Collision|BreakHitResult _outhit))
          (Effects|SpawnEmitteratLocation "/Game/FPS_Weapon_Bundle/Weapons/FX/P_Explosion.P_Explosion" (.Location (Collision|BreakHitResult _outhit)) (Math|Rotator|MakeRotfromX (.Normal (Collision|BreakHitResult _outhit))) (Math|Conversions|ToVector(Float) (Math|Float|MakeLiteralFloat 0.5)) true "AutoRelease")
          (Game|Damage|ApplyPointDamage (.HitActor (Collision|BreakHitResult _outhit)) 5e+01 (.Location (Collision|BreakHitResult _outhit)) _outhit))))
    (else
      (Development|PrintString "Ammo empty!"))))

(event Custom|StartShoot
  (bind _returnvalue (Utilities|Time|SetTimerbyEvent (delegate Custom|Shoot) 0.1 true))
  (Variables|Default|SetShootTimer _returnvalue)
  (CallFunction|Shoot))

(event Custom|StopShoot
  (Utilities|Time|ClearandInvalidateTimerbyHandle (Variables|Default|GetShootTimer)))

(event Custom|Reload
  (Development|PrintString "Reloading!")
  (Utilities|FlowControl|RetriggerableDelay 2.0)
  (Variables|Default|SetAmmo 30)
  (Development|PrintString "Reloaded!")
  (Default|CallOnReloaded 0.0))

(fn ConstructionScript)